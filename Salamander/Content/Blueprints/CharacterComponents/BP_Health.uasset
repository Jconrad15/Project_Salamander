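; BP_Health is a health component for characters that tracks current health and death state.
; Damage subtracts an amount from CurrentHealth, clamping at zero, setting IsDead and returning true when health runs out, otherwise false.
; ReadHealth exposes the current value, and the event graph holds no active logic.
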(fn `Damage`
  (params (DamageAmount :type "Float (double-precision)"))
  (returns (Died :type Boolean))
  (bind _returnvalue (- (`self.CurrentHealth`) DamageAmount))
  (if (<= _returnvalue 0.0)
    (set `self.CurrentHealth` 0.0)
    (set `self.isDead` true)
    (return true)
    (else
      (set `self.CurrentHealth` _returnvalue)
      (return false))))

(fn `ReadHealth`
  (returns (CurrentHealth :type "Float (double-precision)"))
  (return (`self.CurrentHealth`)))