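; Sanity tracker that moves a clamped value between despair (negative) and hubris (positive) based on the sanity volumes currently affecting it.
; Each tick it sums the volumes' rates, with Sane volumes pulling toward zero outside a small dead zone, then applies the total over delta time and prints the result.
; It also supports instant changes, normalized and limit getters, and registration for a sanity-changed callback.
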(event `self.ReceiveTick`
  (params (DeltaSeconds :type "Float (single-precision)"))
  (`self.DetermineSanityRateChange`)
  (`self.UpdateSanity` DeltaSeconds)
  (`KismetSystemLibrary.PrintString` (`KismetStringLibrary.Concat_StrStr` "Sanity: " (`KismetStringLibrary.Conv_DoubleToString` (`self.CurrentSanity`))) true true (struct :`G` 0.66 :`B` 1.0 :`A` 1.0) 0.0))

(fn `DetermineSanityRateChange`
  (locals (RunningTotal :type "Float (double-precision)"))
  (bind _currentsanity (`self.CurrentSanity`))
  (for _array_element (`self.CurrentSanityVolumes`)
    (switch `/Game/Blueprints/SanityMechanic/E_SanityType` (`/Game/Blueprints/SanityMechanic/BP_SanityVolume.SanityType` _array_element)
      (:`NewEnumerator0`
        (bind _sanityratechange (`/Game/Blueprints/SanityMechanic/BP_SanityVolume.SanityRateChange` _array_element))
        ;[1 1 1] Despair
        (set `local.RunningTotal` (- (`local.RunningTotal`) _sanityratechange) :!label _label))
      (:`NewEnumerator1`
        ;[1 1 1] Sane
        (if (> _currentsanity 0.05)
          (goto _label)
          (elif (< _currentsanity -0.05)
            ;[1 1 1] Hubris
            (set `local.RunningTotal` (+ (`local.RunningTotal`) _sanityratechange) :!label _label_2))))
      (:`NewEnumerator2`
        (goto _label_2))))
  (set `self.SanityRateChange` (`local.RunningTotal`)))

(fn `GetMaxSanity`
  (returns (MaxSanity :type "Float (double-precision)"))
  (return (`self.MaxSanity`)))

(fn `GetMinSanity`
  (returns (MinSanity :type "Float (double-precision)"))
  (return (`self.MinSanity`)))

(fn `GetNormalizedSanity`
  (returns (NormalizedSanity :type "Float (double-precision)"))
  (return (/ (+ (`self.CurrentSanity`) (`KismetMathLibrary.Abs` (`self.MinSanity`))) (- (`self.MaxSanity`) (`self.MinSanity`)))))

(fn `InstantChangeSanity`
  (params (SanityChange :type "Float (double-precision)"))
  (bind _output_get (set `self.CurrentSanity` (`KismetMathLibrary.FClamp` (+ SanityChange (`self.CurrentSanity`)) (`self.MinSanity`) (`self.MaxSanity`))))
  (if (!= SanityChange 0.0)
    (`self.cbOnSanityChanged` _output_get)))

(fn `RegisterOnSanityChanged`
  (params (Event :type "Delegate (by ref)"))
  (add `self.cbOnSanityChanged` Event))

(fn `UpdateSanity`
  (params (DeltaSeconds :type "Float (double-precision)"))
  (locals (StartingFrameSanity :type "Float (double-precision)"))
  (bind _currentsanity (`self.CurrentSanity`))
  (set `local.StartingFrameSanity` (`self.CurrentSanity`))
  (set `self.CurrentSanity` (`KismetMathLibrary.FClamp` (+ (* DeltaSeconds (`self.SanityRateChange`)) (`self.CurrentSanity`)) (`self.MinSanity`) (`self.MaxSanity`)))
  ;[1 1 1] Call back function if sanity changed
  (if (!= (`local.StartingFrameSanity`) _currentsanity)
    (`self.cbOnSanityChanged` _currentsanity)))