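; Base enemy character Blueprint that provides patrol points, adjustable walk speed and death on damage.
; On BeginPlay it rebuilds PatrolLocations with its spawn position as the first point, exposed through GetPatrolLocations.
; Any incoming damage is forwarded to BPHealth, and the actor destroys itself when that call returns true.
; UpdateWalkSpeed sets the CharacterMovement max walk speed for callers.
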(event `self.ReceiveBeginPlay`
  (`self.SetStartLocationInPatrol`))

(event `self.ReceiveAnyDamage`
  (params (Damage :type "Float (single-precision)") (DamageType :type "DamageType Object Reference") (InstigatedBy :type "Controller Object Reference") (DamageCauser :type "Actor Object Reference"))
  (bind _died (`/Game/Blueprints/CharacterComponents/BP_Health.Damage` (`self.BP_Health`) Damage))
  (if _died
    (`self.K2_DestroyActor`)))

(fn `GetPatrolLocations`
  (returns (PatrolLocations :type "Array of Vector Structure"))
  (return (`self.PatrolLocations`)))

(fn `SetStartLocationInPatrol`
  (locals (TempPatrolLocations :type "Array of Vector Structure"))
  (set `local.TempPatrolLocations` (`self.PatrolLocations`))
  (`KismetArrayLibrary.Array_Clear` (`self.PatrolLocations`))
  (`KismetArrayLibrary.Array_Add` (`self.PatrolLocations`) (`self.K2_GetActorLocation`))
  (for _array_element (`local.TempPatrolLocations`)
    (`KismetArrayLibrary.Array_Add` (`self.PatrolLocations`) _array_element)))

(fn `UpdateWalkSpeed`
  (params (NewWalkSpeed :type "Float (double-precision)"))
  (set `CharacterMovementComponent.MaxWalkSpeed` NewWalkSpeed (`self.CharacterMovement`)))

(fn `UserConstructionScript`)