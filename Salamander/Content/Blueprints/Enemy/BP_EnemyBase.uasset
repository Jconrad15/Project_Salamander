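; BP_EnemyBase is an enemy base Blueprint that wanders around and can take damage.
; MoveEnemy picks a random reachable point around its current location, runs AI MoveTo, then calls itself again after a pause on success or a brief delay on failure.
; AnyDamage prints a debug string, forwards the damage to BPHealth and destroys the actor when that call returns true.
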(event `self.ReceiveBeginPlay`
  (`self.MoveEnemy`))

(event `MoveEnemy`
  (bind _output_get (set `self.Random Location` (`NavigationSystemV1.K2_GetRandomReachablePointInRadius` (`self.K2_GetActorLocation`) 1000.0 null null)))
  (`|AIMoveTo` self _output_get null
    (:`OnSuccess`
      (`KismetSystemLibrary.Delay` 5.0)
      (`self.MoveEnemy`))
    (:`OnFail`
      (`KismetSystemLibrary.Delay` 0.1)
      (`self.MoveEnemy`))))

(event `self.ReceiveAnyDamage`
  (params (Damage :type "Float (single-precision)") (DamageType :type "DamageType Object Reference") (InstigatedBy :type "Controller Object Reference") (DamageCauser :type "Actor Object Reference"))
  (`KismetSystemLibrary.PrintString` "DamageEvent")
  (bind _died (`/Game/Blueprints/HealthComponent/BP_Health.Damage` (`self.BP_Health`) Damage))
  (if _died
    (`self.K2_DestroyActor`)))

(fn `UserConstructionScript`)