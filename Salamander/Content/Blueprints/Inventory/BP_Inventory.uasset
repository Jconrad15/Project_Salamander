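; Player inventory component that handles looking at and interacting with objects and tracks obtained ingredients.
; Each tick, a box trace ahead of player character 0 updates LookAtActor and shows its message in a WBP_DisplayMessage widget created on BeginPlay.
; The Interact input calls InteractWithMessage on that actor, passing the owning character.
; ObtainIngredient sets a separate boolean for each of three ingredient types: toadstools, scepter and crypt dust.
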(event `self.ReceiveBeginPlay`
  ;[1 1 1] Create Display Message Widget - note probably should be done here
  (bind _returnvalue (`|CreateWidget` "/Game/Blueprints/Inventory/WBP_DisplayMessage.WBP_DisplayMessage_C"))
  (bind _output_get (set `self.DisplayMessage` _returnvalue))
  (`UserWidget.AddToViewport` _output_get 0))

(event `self.ReceiveTick`
  (params (DeltaSeconds :type "Float (single-precision)"))
  (`self.InteractionTrace`))

(event `InputAction|Interact`
  (params (Key :type "Key Structure"))
  (:`Pressed`
    (bind _lookatactor (`self.LookAtActor`)
      (:`then`
        ;[1 1 1] Try trigger interact
        (message `/Game/Blueprints/Inventory/BI_Interact.InteractWith` _lookatactor (cast `/Game/ThirdPerson/Blueprints/BP_ThirdPersonCharacter` (`self.GetOwner`) :!pure true)))
      (:`else`
        (`KismetSystemLibrary.PrintString` "No interactable")))))

(fn `InteractionTrace`
  (locals (InteractionRange :type "Float (single-precision)"))
  (bind _returnvalue (`GameplayStatics.GetPlayerCharacter` 0))
  (bind _returnvalue_2 (`Actor.K2_GetActorLocation` _returnvalue))
  (bind _returnvalue_3 (`Actor.GetActorForwardVector` _returnvalue))
  ;[1 1 1] Create box trace
  (bind (_outhit _returnvalue_4) (`KismetSystemLibrary.BoxTraceSingle` _returnvalue_2 (+ _returnvalue_2 (* _returnvalue_3 (`local.InteractionRange`))) (90.0 90.0 150.0) (`KismetMathLibrary.Conv_VectorToRotator` _returnvalue_3) "TraceTypeQuery3" false (`|MakeArray` (`self.GetOwner`))))
  (if _returnvalue_4
    (bind (_bblockinghit _binitialoverlap _time _distance _location _impactpoint _normal _impactnormal _physmat _hitactor) (`GameplayStatics.BreakHitResult` _outhit))
    ;[1 1 1] Is hit interactable different from last hit interactable?
    (if (!= _hitactor (`self.LookAtActor`))
      (bind _output_get (set `self.LookAtActor` _hitactor))
      ;[1 1 1] Show display message
      (bind _message (message `/Game/Blueprints/Inventory/BI_Interact.LookAt` _output_get))
      (`/Game/Blueprints/Inventory/WBP_DisplayMessage.TriggerShowMessage` (`self.DisplayMessage`) _message))
    (else
      ;[1 1 1] No interactable hit
      (set `self.LookAtActor` null)
      (`/Game/Blueprints/Inventory/WBP_DisplayMessage.TriggerShowMessage` (`self.DisplayMessage`) ""))))

(fn `ObtainIngredient`
  (params (IngredientType :type "/Game/Blueprints/Inventory/ENUM_IngredientType Enum" :default "NewEnumerator0"))
  (switch `/Game/Blueprints/Inventory/ENUM_IngredientType` IngredientType
    (:`NewEnumerator0`
      (set `self.SpectralToadstools` true))
    (:`NewEnumerator1`
      (set `self.ScepterOfTheFallenKing` true))
    (:`NewEnumerator2`
      (set `self.CryptDust` true))))