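; KeyRing is a Blueprint that tracks the keys picked up, stored by ID in CurrentKeys.
; PickupKey adds a new ID to the collection.
; TryUseKey checks for an ID, removes it if present and returns the removal result, so using a key consumes it; otherwise it returns the failed Contains check.
; BeginPlay and Tick are unused.
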(fn `PickupKey`
  (params (NewID :type Byte))
  (`KismetArrayLibrary.Array_Add` (`self.CurrentKeys`) NewID))

(fn `TryUseKey`
  (params (TryID :type Byte))
  (returns (Success :type Boolean))
  (bind _returnvalue (`KismetArrayLibrary.Array_Contains` (`self.CurrentKeys`) TryID))
  (if _returnvalue
    (bind _returnvalue_2 (`KismetArrayLibrary.Array_RemoveItem` (`self.CurrentKeys`) (`local.TryID`)))
    (return _returnvalue_2)
    (else
      (return _returnvalue))))