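; Key-locked door actor that opens when a player holding the matching key walks into it.
; On sphere overlap while locked, it asks the ThirdPersonCharacter's KeyRing to use NeededKeyID, printing a debug message if that fails.
; Opening currently just clears IsLocked and destroys the actor as a placeholder for a later animation.
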(event `self.SphereCollider.OnComponentBeginOverlap`
  (params (OverlappedComponent :type "PrimitiveComponent Object Reference") (OtherActor :type "Actor Object Reference") (OtherComp :type "PrimitiveComponent Object Reference") (OtherBodyIndex :type Integer) (bFromSweep :type Boolean) (SweepResult :type "HitResult Structure (by ref)"))
  (if (`self.IsLocked`)
    ;[1 1 1] Try Unlock
    (bind _asbp_third_person_character (cast `/Game/ThirdPerson/Blueprints/BP_ThirdPersonCharacter` OtherActor))
    (bind _success (`/Game/Blueprints/Keys/KeyRing.TryUseKey` (`/Game/ThirdPerson/Blueprints/BP_ThirdPersonCharacter.KeyRing` _asbp_third_person_character) (`self.NeededKeyID`)))
    (if _success
      (`self.UnlockAndOpenDoor`)
      (else
        (`KismetSystemLibrary.PrintString` "Didn't have correct key in keyring")))))

(fn `UnlockAndOpenDoor`
  ;[1 1 1] Currently just destroy the door to show that it is open.  Can animate it later
  (set `self.IsLocked` false)
  (`self.K2_DestroyActor`))

(fn `UserConstructionScript`)