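; Whitebox dry swamp collision actor that slows the third-person player character while overlapping it.
; On begin overlap it sets the character's MaxWalkSpeed to a third of its current max speed.
; On end overlap it multiplies that speed by only 1.5, so each pass leaves the character at half its previous speed rather than restoring it.
; Both events print debug strings.
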(event `self.ReceiveActorBeginOverlap`
  (params (OtherActor :type "Actor Object Reference"))
  (bind _asbp_third_person_character (cast `/Game/ThirdPerson/Blueprints/BP_ThirdPersonCharacter` OtherActor))
  (bind _charactermovement (`Character.CharacterMovement` _asbp_third_person_character))
  (set `CharacterMovementComponent.MaxWalkSpeed` (/ (`MovementComponent.GetMaxSpeed` _charactermovement) 3.0) _charactermovement)
  (`KismetSystemLibrary.PrintString` "SLOW"))

(event `self.ReceiveActorEndOverlap`
  (params (OtherActor :type "Actor Object Reference"))
  (bind _asbp_third_person_character (cast `/Game/ThirdPerson/Blueprints/BP_ThirdPersonCharacter` OtherActor))
  (bind _charactermovement (`Character.CharacterMovement` _asbp_third_person_character))
  (set `CharacterMovementComponent.MaxWalkSpeed` (* (`MovementComponent.GetMaxSpeed` _charactermovement) 1.5) _charactermovement)
  (`KismetSystemLibrary.PrintString` "REGULAR"))

(fn `UserConstructionScript`)