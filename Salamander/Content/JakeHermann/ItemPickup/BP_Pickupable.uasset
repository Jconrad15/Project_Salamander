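; BP_Pickupable is a component that lets its owning actor be picked up, carried and dropped by the player.
; Pickup disables physics on all the owner's primitive components and sets IsPickedUp; TryDrop reverses both and returns whether a drop happened.
; While held, Tick moves the owner by swept transforms to the HeldItemLocation from the player character's BP_PickerUpper, zeroing rotation and preserving scale.
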(event `self.ReceiveBeginPlay`
  (set `self.Owner` (`self.GetOwner`)))

(event `self.ReceiveTick`
  (params (DeltaSeconds :type "Float (single-precision)"))
  (bind _returnvalue (`self.GetOwner`))
  (if (`self.IsPickedUp`)
    (bind _asbp_third_person_character (cast `/Game/ThirdPerson/Blueprints/BP_ThirdPersonCharacter` (`GameplayStatics.GetPlayerCharacter` 0)))
    (bind _helditemlocation (`/Game/JakeHermann/ItemPickup/BP_PickerUpper.HeldItemLocation` (`Actor.GetComponentByClass` _asbp_third_person_character "/Game/JakeHermann/ItemPickup/BP_PickerUpper.BP_PickerUpper_C")))
    (`Actor.K2_SetActorLocation` _returnvalue _helditemlocation true false)
    (`SceneComponent.K2_SetWorldTransform` (`Actor.RootComponent` (`self.Owner`)) (`KismetMathLibrary.MakeTransform` _helditemlocation (struct) (`Actor.GetActorScale3D` _returnvalue)) true true)))

(fn `Pickup`
  (`KismetSystemLibrary.PrintString` "Pick up" false)
  (if (`self.IsPickedUp`)
    (`KismetSystemLibrary.PrintString` "Errror" false)
    (else
      (`self.Toggle Physics` false)
      (set `self.IsPickedUp` true))))

(fn `Toggle Physics`
  (params (TurnOn :type Boolean))
  (for _array_element (`Actor.K2_GetComponentsByClass` (`self.Owner`) "/Script/Engine.PrimitiveComponent")
    (`PrimitiveComponent.SetSimulatePhysics` _array_element TurnOn))
  (`KismetSystemLibrary.PrintString` (`KismetStringLibrary.Concat_StrStr` "Physics is on: " (`KismetStringLibrary.Conv_BoolToString` TurnOn)) false))

(fn `TryDrop`
  (returns (wasDropped :type Boolean))
  (if (`self.IsPickedUp`)
    (set `self.IsPickedUp` false)
    (`self.Toggle Physics` true)
    (`KismetSystemLibrary.PrintString` "Dropped" false true (struct :`R` 0.167905 :`G` 1.0 :`B` 0.227356 :`A` 1.0))
    (return true)
    (else
      (return false))))