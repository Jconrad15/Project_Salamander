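; BP_PickerUpper lets its owning third-person character pick up and release items with the left mouse button.
; Pressing runs a debug-drawn capsule trace from the follow camera, stores the hit actor as HeldItem and calls Pickup on its BP_Pickupable component.
; Releasing calls TryDrop and clears HeldItem on success.
; Tick updates HeldItemLocation at a hold distance ahead of the camera, without moving the item itself.
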(event `Key|LeftMouseButton`
  (params (Key :type "Key Structure"))
  (:`Pressed`
    ;[0.08333 0.08333 0.08333] Pickup Item
    ;;[1 1 1] Create trace
    (bind _asbp_third_person_character (cast `/Game/ThirdPerson/Blueprints/BP_ThirdPersonCharacter` (`self.GetOwner`)))
    (bind _followcamera (`/Game/ThirdPerson/Blueprints/BP_ThirdPersonCharacter.FollowCamera` _asbp_third_person_character))
    (bind _returnvalue (`SceneComponent.K2_GetComponentLocation` _followcamera))
    (bind (_outhit _returnvalue_2) (`KismetSystemLibrary.CapsuleTraceSingle` _returnvalue (+ _returnvalue (* (`SceneComponent.GetForwardVector` _followcamera) (`self.InteractionRange`))) 30.0 15.0 "TraceTypeQuery3" false (`|MakeArray` (`self.GetOwner`)) "ForDuration"))
    (if _returnvalue_2
      ;;[1 1 1] Set held item
      (bind _output_get (set `self.HeldItem` (`.HitActor` (`GameplayStatics.BreakHitResult` _outhit))))
      (bind _returnvalue_3 (`Actor.GetComponentByClass` _output_get "/Game/JakeHermann/ItemPickup/BP_Pickupable.BP_Pickupable_C"))
      ;;[1 1 1] Trigger pickup
      (`/Engine/EditorBlueprintResources/StandardMacros.IsValid` _returnvalue_3
        (:`Is Valid`
          (`/Game/JakeHermann/ItemPickup/BP_Pickupable.Pickup` _returnvalue_3)
          (`KismetSystemLibrary.PrintString` "Picked up" false))
        (:`Is Not Valid`
          (`KismetSystemLibrary.PrintString` "Hit item has not Pickupable component" false)))
      (else
        ;;[1 1 1] No interactable hit
        (set `self.HeldItem` null)
        (`KismetSystemLibrary.PrintString` "No interactable hit"))))
  (:`Released`
    ;[1 1 1] Drop Item
    (bind _helditem (`self.HeldItem`)
      (:`then`
        (bind _wasdropped (`/Game/JakeHermann/ItemPickup/BP_Pickupable.TryDrop` (`Actor.GetComponentByClass` _helditem "/Game/JakeHermann/ItemPickup/BP_Pickupable.BP_Pickupable_C")))
        (if _wasdropped
          (set `self.HeldItem` null)
          (`KismetSystemLibrary.PrintString` "Held item is now set null" false)
          (else
            (`KismetSystemLibrary.PrintString` "Error"))))
      (:`else`
        (`KismetSystemLibrary.PrintString` "No held item to release" false)))))

(event `self.ReceiveTick`
  (params (DeltaSeconds :type "Float (single-precision)"))
  (bind _asbp_third_person_character (cast `/Game/ThirdPerson/Blueprints/BP_ThirdPersonCharacter` (`self.GetOwner`)))
  (bind _followcamera (`/Game/ThirdPerson/Blueprints/BP_ThirdPersonCharacter.FollowCamera` _asbp_third_person_character))
  (set `self.HeldItemLocation` (+ (`SceneComponent.K2_GetComponentLocation` _followcamera) (* (`SceneComponent.GetForwardVector` _followcamera) (`self.Hold Distance`)))))