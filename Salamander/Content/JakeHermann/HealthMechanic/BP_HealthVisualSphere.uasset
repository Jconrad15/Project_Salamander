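; BP_HealthVisualSphere is a child actor that displays its parent actor's health as five colored spheres.
; On BeginPlay it finds the parent's BP_Health component and creates a dynamic material for each sphere.
; Each tick, the health ratio samples a color curve for the materials' base color and a float curve that decides how many spheres stay visible.
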(event `self.ReceiveBeginPlay`
  (set `self.HealthComponent` (`self.GetComponentByClass` (`self.GetParentActor`) "/Game/JakeHermann/HealthMechanic/BP_Health.BP_Health_C"))
  (`self.CreateSphereArray`)
  (for _array_element (`self.Spheres`)
    (bind _returnvalue (`PrimitiveComponent.CreateDynamicMaterialInstance` _array_element 0 null "None"))
    (`KismetArrayLibrary.Array_AddUnique` (`self.Material`) _returnvalue)))

(event `self.ReceiveTick`
  (params (DeltaSeconds :type "Float (single-precision)"))
  (`self.Set Sphere Visuals`))

(fn `CreateSphereArray`
  (`KismetArrayLibrary.Array_AddUnique` (`self.Spheres`) (`self.Sphere`))
  (`KismetArrayLibrary.Array_AddUnique` (`self.Spheres`) (`self.Sphere1`))
  (`KismetArrayLibrary.Array_AddUnique` (`self.Spheres`) (`self.Sphere2`))
  (`KismetArrayLibrary.Array_AddUnique` (`self.Spheres`) (`self.Sphere3`))
  (`KismetArrayLibrary.Array_AddUnique` (`self.Spheres`) (`self.Sphere4`)))

(fn `Set Sphere Visuals`
  (bind _healthcomponent (`self.HealthComponent`))
  (bind _healthcomponent_2 (`self.HealthComponent`))
  (for _array_element (`self.Material`)
    (`MaterialInstanceDynamic.SetVectorParameterValue` _array_element "Base Color" (`CurveLinearColor.GetLinearColorValue` (`self.HealthSphereColorCurve`) (/ (`/Game/JakeHermann/HealthMechanic/BP_Health.GetHealth` _healthcomponent_2) (`/Game/JakeHermann/HealthMechanic/BP_Health.GetMaxHealth` _healthcomponent_2))))
    (for (_array_element_2 _array_index) (`self.Spheres`)
      (if (< (`CurveFloat.GetFloatValue` (`self.HealthSphereCount`) (/ (`/Game/JakeHermann/HealthMechanic/BP_Health.GetHealth` _healthcomponent) (`/Game/JakeHermann/HealthMechanic/BP_Health.GetMaxHealth` _healthcomponent))) _array_index)
        (`SceneComponent.SetVisibility` _array_element_2 false false)
        (else
          (`SceneComponent.SetVisibility` _array_element_2 true false))))))

(fn `UserConstructionScript`)