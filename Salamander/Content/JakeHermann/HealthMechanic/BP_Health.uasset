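; BP_Health tracks health, clamped between zero and a maximum, and flags death when it reaches zero.
; Each tick it loops over the current health-change volumes, summing their rates and applying the running total scaled by delta time inside the loop, so earlier volumes count repeatedly.
; All changes go through InstantHealthChange, which runs the death check; Die currently only prints a debug message.
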(event `self.ReceiveTick`
  (params (DeltaSeconds :type "Float (single-precision)"))
  (`self.Continuous Health Change` DeltaSeconds))

(event `Die`
  (`KismetSystemLibrary.PrintString` "DeadNow" true true (struct :`R` 0.760417 :`B` 0.006723 :`A` 1.0) 0.05))

(fn `Continuous Health Change`
  (params (DeltaSeconds :type "Float (double-precision)"))
  (locals (RunningTotal :type "Float (double-precision)"))
  ;[1 1 1] Determine rate of change from health volumes
  (for _array_element (`self.CurrentHealthChangeVolumes`)
    (bind _output_get (set `local.RunningTotal` (+ (`/Game/JakeHermann/HealthMechanic/BP_HealthChangeVolume.HealthRateChange` _array_element) (`local.RunningTotal`))))
    (`self.InstantHealthChange` (* _output_get DeltaSeconds))))

(fn `DeadCheck`
  (if (== (`self.Health`) 0.0)
    (set `self.isDead` true)
    (`self.Die`)))

(fn `GetHealth`
  (returns (Health :type "Float (double-precision)"))
  (return (`self.Health`)))

(fn `GetMaxHealth`
  (returns (MaxHealth :type "Float (double-precision)"))
  (return (`self.MaxHealth`)))

(fn `InstantHealthChange`
  (params (Amount :type "Float (double-precision)"))
  (set `self.Health` (`KismetMathLibrary.FClamp` (+ Amount (`self.Health`)) 0.0 (`self.MaxHealth`)))
  (`self.DeadCheck`))