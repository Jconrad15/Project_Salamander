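; BP_SpikeTrap is a one-shot floor trap that raises spikes when the third-person character enters its box trigger.
; The first overlap snaps SpikePlane to MaxHeight, sets IsTriggered (never reset here) and calls ApplyDamage, a placeholder that only prints a debug message.
; When the character leaves the box, CapsuleCollision is enabled for query and physics and set to block the Visibility channel.
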(event `self.BoxCollision.OnComponentBeginOverlap`
  (params (OverlappedComponent :type "PrimitiveComponent Object Reference") (OtherActor :type "Actor Object Reference") (OtherComp :type "PrimitiveComponent Object Reference") (OtherBodyIndex :type Integer) (bFromSweep :type Boolean) (SweepResult :type "HitResult Structure (by ref)"))
  ;[1 1 1] Currently triggers on third person character,
  ; but can also have spikes hurt enemies
  (cast `/Game/ThirdPerson/Blueprints/BP_ThirdPersonCharacter` OtherActor)
  (if (not (`self.isTriggered`))
    (`self.TriggerSpikes`)
    (`self.ApplyDamage`)))

(event `self.BoxCollision.OnComponentEndOverlap`
  (params (OverlappedComponent :type "PrimitiveComponent Object Reference") (OtherActor :type "Actor Object Reference") (OtherComp :type "PrimitiveComponent Object Reference") (OtherBodyIndex :type Integer))
  (cast `/Game/ThirdPerson/Blueprints/BP_ThirdPersonCharacter` OtherActor)
  (`self.EnableSpikeCollision`))

(fn `ApplyDamage`
  (`KismetSystemLibrary.PrintString` "Damage Player Here" true true (struct :`R` 0.864583 :`G` 0.01501 :`A` 1.0) 5.0))

(fn `EnableSpikeCollision`
  (bind _capsulecollision (`self.CapsuleCollision`))
  (`PrimitiveComponent.SetCollisionResponseToChannel` _capsulecollision "ECC_Visibility" "ECR_Block")
  (`PrimitiveComponent.SetCollisionEnabled` _capsulecollision "QueryAndPhysics"))

(fn `TriggerSpikes`
  (`SceneComponent.K2_SetRelativeLocation` (`self.SpikePlane`) (`KismetMathLibrary.MakeVector` 0.0 0.0 (`self.MaxHeight`)) false false)
  (set `self.isTriggered` true))

(fn `UserConstructionScript`)