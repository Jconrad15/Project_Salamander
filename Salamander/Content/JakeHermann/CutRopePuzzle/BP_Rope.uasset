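; BP_Rope is a puzzle rope that gets cut when a BP_Projectile_Basic hits its cylinder.
; The hit height is centered on the cylinder's axis, then sphere traces along the actor's up and down directions look for each half's endpoint.
; It spawns two BP_CutRope actors at the cut, passing each an end offset and cable length from its trace, then destroys itself.
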(event `self.Cylinder.OnComponentHit`
  (params (HitComponent :type "PrimitiveComponent Object Reference") (OtherActor :type "Actor Object Reference") (OtherComp :type "PrimitiveComponent Object Reference") (NormalImpulse :type "Vector Structure") (Hit :type "HitResult Structure (by ref)"))
  (cast `/Game/Projectiles/BP_Projectile_Basic` OtherActor)
  (`self.CreateCutRope` (`.Location` (`GameplayStatics.BreakHitResult` Hit))))

(fn `CreateCutRope`
  (params (cutLocation :type "Vector Structure"))
  (locals (CenteredCutLocation :type "Vector Structure"))
  (bind _centeredcutlocation (`local.CenteredCutLocation`))
  (bind _centeredcutlocation_2 (`local.CenteredCutLocation`))
  (bind (_returnvalue_x _returnvalue_y) (`KismetMathLibrary.BreakVector` (`SceneComponent.K2_GetComponentLocation` (`self.Cylinder`))))
  ;[1 1 1] Center cut location to object location
  (bind _output_get (set `local.CenteredCutLocation` (`KismetMathLibrary.MakeVector` _returnvalue_x _returnvalue_y cutLocation_Z)))
  ;[1 1 1] Create top half
  (bind _outhit (`KismetSystemLibrary.SphereTraceSingle` _output_get (+ _output_get (* (`self.GetActorUpVector`) (`self.MaxTraceDistance`))) 1.0 "TraceTypeQuery4"))
  (bind (_bblockinghit _binitialoverlap _time _distance _location) (`GameplayStatics.BreakHitResult` _outhit))
  (`|SpawnActorFromClass` "/Game/JakeHermann/CutRopePuzzle/BP_CutRope.BP_CutRope_C" (`KismetMathLibrary.MakeTransform` (`local.CenteredCutLocation`)) "Undefined" "MultiplyWithRoot" null (- _location _centeredcutlocation_2) (`KismetMathLibrary.Vector_Distance` _centeredcutlocation_2 _location) null)
  ;[1 1 1] Create bottom half
  (bind _outhit_2 (`KismetSystemLibrary.SphereTraceSingle` (`local.CenteredCutLocation`) (- (`local.CenteredCutLocation`) (* (`self.GetActorUpVector`) (`self.MaxTraceDistance`))) 1.0 "TraceTypeQuery4"))
  (bind (_bblockinghit_2 _binitialoverlap_2 _time_2 _distance_2 _location_2) (`GameplayStatics.BreakHitResult` _outhit_2))
  (`|SpawnActorFromClass` "/Game/JakeHermann/CutRopePuzzle/BP_CutRope.BP_CutRope_C" (`KismetMathLibrary.MakeTransform` (`local.CenteredCutLocation`)) "Undefined" "MultiplyWithRoot" null (- _location_2 _centeredcutlocation) (`KismetMathLibrary.Vector_Distance` _centeredcutlocation _location_2) null)
  (`self.K2_DestroyActor`))

(fn `UserConstructionScript`)