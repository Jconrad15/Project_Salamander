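; BP_SanityVolume is a box trigger volume for the sanity mechanic that tracks when a third-person character is inside it.
; On begin overlap, it adds itself uniquely to the CurrentSanityVolumes list on the character's BP_Sanity component, and on end overlap it removes itself.
; The volume holds no sanity logic of its own and only maintains that list, which supports overlapping volumes.
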(event `self.Box.OnComponentBeginOverlap`
  (params (OverlappedComponent :type "PrimitiveComponent Object Reference") (OtherActor :type "Actor Object Reference") (OtherComp :type "PrimitiveComponent Object Reference") (OtherBodyIndex :type Integer) (bFromSweep :type Boolean) (SweepResult :type "HitResult Structure (by ref)"))
  (bind _asbp_third_person_character (cast `/Game/ThirdPerson/Blueprints/BP_ThirdPersonCharacter` OtherActor))
  (`KismetArrayLibrary.Array_AddUnique` (`/Game/JakeHermann/SanityMechanic/BP_Sanity.CurrentSanityVolumes` (`self.GetComponentByClass` _asbp_third_person_character "/Game/JakeHermann/SanityMechanic/BP_Sanity.BP_Sanity_C")) self))

(event `self.Box.OnComponentEndOverlap`
  (params (OverlappedComponent :type "PrimitiveComponent Object Reference") (OtherActor :type "Actor Object Reference") (OtherComp :type "PrimitiveComponent Object Reference") (OtherBodyIndex :type Integer))
  (bind _asbp_third_person_character (cast `/Game/ThirdPerson/Blueprints/BP_ThirdPersonCharacter` OtherActor))
  (`KismetArrayLibrary.Array_RemoveItem` (`/Game/JakeHermann/SanityMechanic/BP_Sanity.CurrentSanityVolumes` (`self.GetComponentByClass` _asbp_third_person_character "/Game/JakeHermann/SanityMechanic/BP_Sanity.BP_Sanity_C")) self))

(fn `UserConstructionScript`)