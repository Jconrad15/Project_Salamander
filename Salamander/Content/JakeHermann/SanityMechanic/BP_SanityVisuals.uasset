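; Component on the third-person character that turns its current sanity into camera, screen and heartbeat audio feedback, and creates the sanity widget.
; Each tick, curves keyed on sanity drive the follow camera's post-process settings, boom length and roll.
; A looping timer, sped up or slowed by sanity, samples a heartbeat curve to pulse a post-process intensity and audio volume together.
; Debug code prints values on screen and cycles heartbeat sounds by key.
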(event EventBeginPlay
  (CallFunction|FindComponents)
  (bind _returnvalue (UserInterface|CreateWidget "/Game/JakeHermann/SanityMechanic/WBP_SanityWidget.WBP_SanityWidget_C"))
  (UserInterface|Viewport|AddtoViewport _returnvalue 0)
  (Audio|Components|Audio|Play (Variables|Default|GetAudio) 0.0))

(event EventTick
  (params (DeltaSeconds :type Float%20%28single-precision%29))
  (bind _vignette (CallFunction|DetermineVignette))
  (bind _filmgrain (CallFunction|DetermineFilmGrain))
  (bind _dirtmaskintensity (CallFunction|DetermineDirtMask))
  (bind _motionblur (CallFunction|DetermineMotionBlur))
  (bind _saturation (CallFunction|DetermineSaturation))
  (bind _contrast (CallFunction|DetermineContrast))
  (bind (_x _y _z _w) (Math|Vector4|BreakVector4 _saturation))
  (bind (_x_2 _y_2 _z_2 _w_2) (Math|Vector4|BreakVector4 _contrast))
  (Variables|Default|SetNormalized%20Sanity (Default|GetNormalizedSanity (Variables|Default|GetBP_Sanity)))
  (bind _heartbeatvalue (CallFunction|DetermineHeartbeat DeltaSeconds))
  (Utilities|Struct|SetmembersinPostProcessSettings (Variables|/Script/Engine.CameraComponent|GetPostProcessSettings (Variables|Default|GetFollowCamera)) _saturation _contrast _heartbeatvalue (Variables|Default|GetDirtMaskTex) _dirtmaskintensity _vignette _filmgrain _motionblur)
  (CallFunction|SetCameraDistance)
  (CallFunction|TiltCamera)
  ;[1 1 1] Debug: display camera values
  (Development|PrintString (Utilities|String|Append "Vignette: " (Utilities|String|ToString(Float) _vignette)) true true "(R=1.000000,G=0.208059,B=0.227956,A=1.000000)" 0.0)
  (Development|PrintString (Utilities|String|Append "Film grain: " (Utilities|String|ToString(Float) _filmgrain)) true true "(R=1.000000,G=0.208059,B=0.227956,A=1.000000)" 0.0)
  (Development|PrintString (Utilities|String|Append "Saturation: " (Utilities|String|ToString(Float) _x) ", " (Utilities|String|ToString(Float) _y) ", " (Utilities|String|ToString(Float) _z) ", " (Utilities|String|ToString(Float) _w)) true true "(R=1.000000,G=0.993623,B=0.178205,A=1.000000)" 0.0)
  (Development|PrintString (Utilities|String|Append "Contrast: " (Utilities|String|ToString(Float) _x_2) ", " (Utilities|String|ToString(Float) _y_2) ", " (Utilities|String|ToString(Float) _z_2) ", " (Utilities|String|ToString(Float) _w_2)) true true "(R=1.000000,G=0.993623,B=0.178205,A=1.000000)" 0.0)
  (Development|PrintString (Utilities|String|Append "Motion blur intensity: " (Utilities|String|ToString(Float) _motionblur)) true true "(R=1.000000,G=0.993623,B=0.178205,A=1.000000)" 0.0)
  (Development|PrintString (Utilities|String|Append "Dirt Mask Intensity: " (Utilities|String|ToString(Float) _dirtmaskintensity)) true true "(R=1.000000,G=0.993623,B=0.178205,A=1.000000)" 0.0))

(event Input|KeyboardEvents|DebugKeyQ
  (params (Key :type Key%20Structure :default "None") (ActionValue :type Input%20Action%20Value%20Structure))
  (bind _audio (Variables|Default|GetAudio))
  (bind _debugheartbeatsounds (Variables|Default|GetDebugHeartbeatSounds))
  ;[1 1 1] Debug - Switch between heartbeat sounds
  (:Pressed
    (bind _result (Math|Integer|IncrementInt (Variables|Default|GetSoundIndex))
      (:%20%20
        (if (>= _result (Utilities|Array|Length _debugheartbeatsounds))
          (Variables|Default|SetSoundIndex 0))
        (Audio|Components|Audio|SetSound _audio (Utilities|Array|Get(acopy) _debugheartbeatsounds _result))
        (Audio|Components|Audio|Play _audio 0.0)
        (Development|PrintString (Utilities|GetObjectName (Utilities|Array|Get(acopy) _debugheartbeatsounds _result)) true true "(R=0.281076,G=0.890625,B=0.159832,A=1.000000)" 3.0)))))

(fn FindComponents
  (bind _asbp_third_person_character (Utilities|Casting|CastToBP_ThirdPersonCharacter (Components|GetOwner)))
  (Utilities|FlowControl|Sequence
    (:then_0
      (Variables|Default|SetFollowCamera (Variables|/Game/ThirdPerson/Blueprints/BP_ThirdPersonCharacter.BP_ThirdPersonCharacter_C|GetCamera_Follow _asbp_third_person_character)))
    (:then_1
      (Variables|Default|SetCameraBoom (Variables|/Game/ThirdPerson/Blueprints/BP_ThirdPersonCharacter.BP_ThirdPersonCharacter_C|GetSpringArm_Camera_Follow _asbp_third_person_character)))
    (:then_2
      (Variables|Default|SetBP_Sanity (Variables|/Game/ThirdPerson/Blueprints/BP_ThirdPersonCharacter.BP_ThirdPersonCharacter_C|GetBP_Sanity _asbp_third_person_character)))
    (:then_3
      (bind _output_get (Variables|Default|SetAudio (Variables|/Game/ThirdPerson/Blueprints/BP_ThirdPersonCharacter.BP_ThirdPersonCharacter_C|GetHeartbeatAudio _asbp_third_person_character)))
      (Audio|Components|Audio|SetSound _output_get (Utilities|Array|Get(acopy) (Variables|Default|GetDebugHeartbeatSounds))))))

(fn DetermineSaturation
  (bind _saturationcurve (Variables|Default|GetSaturationCurve))
  (bind _bp_sanity (Variables|Default|GetBP_Sanity))
  (bind _currentsanity (Variables|/Game/JakeHermann/SanityMechanic/BP_Sanity.BP_Sanity_C|GetCurrentSanity _bp_sanity))
  (bind _returnvalue (Math|Curves|GetLinearColorValue _saturationcurve _currentsanity))
  (bind (_r _g _b _a) (Utilities|Struct|BreakLinearColor _returnvalue))
  (return (Math|Vector4|MakeVector4 _r _g _b _a)))

(fn DetermineContrast
  (bind _contrastcurve (Variables|Default|GetContrastCurve))
  (bind _bp_sanity (Variables|Default|GetBP_Sanity))
  (bind _currentsanity (Variables|/Game/JakeHermann/SanityMechanic/BP_Sanity.BP_Sanity_C|GetCurrentSanity _bp_sanity))
  (bind _returnvalue (Math|Curves|GetLinearColorValue _contrastcurve _currentsanity))
  (bind (_r _g _b _a) (Utilities|Struct|BreakLinearColor _returnvalue))
  (return (Math|Vector4|MakeVector4 _r _g _b _a)))

(fn DetermineVignette
  (return (Math|Curves|GetFloatValue (Variables|Default|GetVignetteIntensityCurve) (Variables|/Game/JakeHermann/SanityMechanic/BP_Sanity.BP_Sanity_C|GetCurrentSanity (Variables|Default|GetBP_Sanity)))))

(fn DetermineFilmGrain
  (return (Math|Curves|GetFloatValue (Variables|Default|GetFilmIntensityCurve) (Variables|/Game/JakeHermann/SanityMechanic/BP_Sanity.BP_Sanity_C|GetCurrentSanity (Variables|Default|GetBP_Sanity)))))

(fn DetermineDirtMask
  (return (Math|Curves|GetFloatValue (Variables|Default|GetDirtMaskIntensityCurve) (Variables|/Game/JakeHermann/SanityMechanic/BP_Sanity.BP_Sanity_C|GetCurrentSanity (Variables|Default|GetBP_Sanity)))))

(fn DetermineHeartbeat
  (params (DeltaSeconds :type Float%20%28double-precision%29))
  (bind _bp_sanity (Variables|Default|GetBP_Sanity))
  (bind _bp_sanity_2 (Variables|Default|GetBP_Sanity))
  (bind _heartbeatintensitycurve (Variables|Default|GetHeartbeatIntensityCurve))
  (bind _heartbeathertzcurve (Variables|Default|GetHeartbeatHertzCurve))
  (bind _currentsanity (Variables|/Game/JakeHermann/SanityMechanic/BP_Sanity.BP_Sanity_C|GetCurrentSanity _bp_sanity))
  (bind _currentsanity_2 (Variables|/Game/JakeHermann/SanityMechanic/BP_Sanity.BP_Sanity_C|GetCurrentSanity _bp_sanity_2))
  (bind _returnvalue (Math|Curves|GetFloatValue _heartbeatintensitycurve _currentsanity))
  (bind _returnvalue_2 (Math|Curves|GetFloatValue _heartbeathertzcurve _currentsanity_2))
  ;[1 1 1] Update Time
  (bind _output_get (Variables|Default|SetTime (+ (Variables|Default|GetTime) (* DeltaSeconds _returnvalue_2))))
  (if (> _output_get 1.0)
    (Variables|Default|SetTime 0.0))
  ;[1 1 1] Heartbeat Audio
  (Audio|Components|Audio|SetVolumeMultiplier (Variables|Default|GetAudio) (- (* _returnvalue (Math|Curves|GetFloatValue (Variables|Default|GetHeartbeatCurve) (Variables|Default|GetTime))) 0.2) :!class /Script/Engine.AudioComponent)
  (Utilities|FlowControl|Sequence
    (:then_0
      ;[1 1 1] Debug info
      (Development|PrintString (Utilities|String|Append "Heartbeat intensity: " (Utilities|String|ToString(Float) _returnvalue)) true true "(R=0.463542,G=0.009554,B=0.018777,A=1.000000)" 0.0)
      (Development|PrintString (Utilities|String|Append "Heartbeat speed (Hz): " (Utilities|String|ToString(Float) _returnvalue_2)) true true "(R=0.463542,G=0.009554,B=0.018777,A=1.000000)" 0.0))
    (:then_1
      (return (* _returnvalue (Math|Curves|GetFloatValue (Variables|Default|GetHeartbeatCurve) (Variables|Default|GetTime)))))))

(fn DetermineMotionBlur
  (return (Math|Curves|GetFloatValue (Variables|Default|GetMotionBlurCurve) (Variables|/Game/JakeHermann/SanityMechanic/BP_Sanity.BP_Sanity_C|GetCurrentSanity (Variables|Default|GetBP_Sanity)))))

(fn SetCameraDistance
  (Variables|/Script/Engine.SpringArmComponent|SetTargetArmLength (Variables|Default|GetCameraBoom) (Math|Curves|GetFloatValue (Variables|Default|GetCameraDistanceCurve) (Variables|/Game/JakeHermann/SanityMechanic/BP_Sanity.BP_Sanity_C|GetCurrentSanity (Variables|Default|GetBP_Sanity)))))

(fn TiltCamera
  (Transformation|SetRelativeRotation (Variables|Default|GetFollowCamera) (Math|Rotator|MakeRotator (Math|Curves|GetFloatValue (Variables|Default|GetCameraTiltCurve) (Variables|/Game/JakeHermann/SanityMechanic/BP_Sanity.BP_Sanity_C|GetCurrentSanity (Variables|Default|GetBP_Sanity))) 0.0 0.0) false false))